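; Player spaceship pawn with six-direction flight, mouse look, sprint and laser fire.
; Tick turns key flags into movement input, banks the body when strafing and sphere-traces from the camera to aim and update the HUD.
; A looping timer drains or regenerates stamina, while a timeline scales thrusters and FOV during sprint.
; Held fire repeats through a cooldown-reset DoOnce, launching bullets toward the target from one or alternating muzzles by WeaponLevel.
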(event Custom|StartSprintEffect
  ;[1 1 1] Sprint Effects Timeline
  (bind _sprint_alpha (Timeline|TL_Sprint Play)
    (:Update
      (Transformation|SetWorldScale3D (Variables|Default|GetP_Thruster1) (Math|Vector|Lerp(Vector) "0.250000,0.500000,0.500000" "0.500000,0.500000,1.500000" _sprint_alpha))
      (Camera|SetFieldOfView (Variables|Default|GetCamera) (Math|Float|Lerp 9e+01 1.1e+02 _sprint_alpha)))))

(event Custom|StopSprintEffect
  ;[1 1 1] Sprint Effects Timeline
  (bind _sprint_alpha (Timeline|TL_Sprint Reverse)
    (:Update
      (Transformation|SetWorldScale3D (Variables|Default|GetP_Thruster1) (Math|Vector|Lerp(Vector) "0.250000,0.500000,0.500000" "0.500000,0.500000,1.500000" _sprint_alpha))
      (Camera|SetFieldOfView (Variables|Default|GetCamera) (Math|Float|Lerp 9e+01 1.1e+02 _sprint_alpha)))))

(event Custom|StartTimers
  ;[1 1 1] Timers
  (bind _returnvalue (Utilities|Time|SetTimerbyEvent (delegate Custom|StaminaRegeneration) 1.0 true))
  (Variables|Movement|SetStaminaTimerHandle _returnvalue))

(event Custom|StaminaRegeneration
  (bind _maxstamina (Variables|Movement|GetMaxStamina))
  ;[1 1 1] Timers
  (bind _output_get (Variables|Movement|SetCurrentStamina (Math|Float|Clamp(Float) (Math|Float|SelectFloat (- (Variables|Movement|GetCurrentStamina) (Variables|Movement|GetStaminaConsumptionValue)) (+ (Variables|Movement|GetCurrentStamina) (Variables|Movement|GetStaminaRegenerationValue)) (Variables|Movement|GetIs_Sprinting)) 0.0 _maxstamina)))
  (Default|UpdateStaminaPercent (Variables|Default|GetWG_Gameplay_Ref) (/ _output_get _maxstamina))
  (Utilities|FlowControl|Sequence
    (:then_0
      (if (== (Variables|Movement|GetCurrentStamina) 0.0)
        (CallFunction|StopSprinting)))
    (:then_1
      (if (== (Variables|Movement|GetCurrentStamina) (Variables|Movement|GetMaxStamina))
        (Utilities|Time|PauseTimerbyHandle (Variables|Movement|GetStaminaTimerHandle))))))

(event Custom|LaserShoot
  ;[1 1 1] Laser Mechanics
  (Utilities|FlowControl|DoOnce false
    (:Completed
      (Utilities|FlowControl|Sequence
        (:then_0
          (Audio|PlaySound2D "/Game/Sounds/617034__d4xx__laser-shot_Cue.617034__d4xx__laser-shot_Cue" 1.0 1.0 0.0 0 0)
          (Utilities|FlowControl|Delay (Variables|Shooting|GetLaserCooldown))
          (CallFunction|ResetLaser)
          (if (Variables|Shooting|GetIsShooting)
            (CallFunction|LaserShoot)))
        (:then_1
          (switch int (Variables|Shooting|GetWeaponLevel)
            (:0
              (CallFunction|SpawnLaser (Variables|Default|GetMuzzle1)))
            (:1
              (bind _isa (Utilities|FlowControl|FlipFlop)
                (:A
                  _)
                (:B
                  _))
              (CallFunction|SpawnLaser (select _isa (Variables|Default|GetMuzzle3) (Variables|Default|GetMuzzle2))))))))))

(event Custom|ResetLaser
  ;[1 1 1] Laser Mechanics
  (Utilities|FlowControl|DoOnce false) ; enters at Reset
)

(event EventBeginPlay
  (Pawn|Possess (Game|GetPlayerController 0) self)
  (CallFunction|SetDefaults)
  (Utilities|FlowControl|Sequence
    (:then_0
      ;[1 1 1] Create Widget Gameplay
      (bind _returnvalue (UserInterface|CreateWidget "/Game/UI/WG_Gameplay.WG_Gameplay_C" (Game|GetPlayerController 0)))
      (bind _output_get (Variables|Default|SetWG_Gameplay_Ref _returnvalue))
      (UserInterface|Viewport|AddtoViewport _output_get 0)
      (Default|UpdateStaminaPercent (Variables|Default|GetWG_Gameplay_Ref) (/ (Variables|Movement|GetCurrentStamina) (Variables|Movement|GetMaxStamina))))
    (:then_1
      (CallFunction|StartTimers))))

(event Collision|EventActorBeginOverlap
  (params (OtherActor :type Actor%20Object%20Reference)))

(event EventTick
  (params (DeltaSeconds :type Float%20%28single-precision%29))
  (Utilities|FlowControl|Sequence
    (:then_0
      ;[1 1 1] Movement
      (Class|PawnMovementComponent|AddInputVector (Variables|Default|GetFloatingPawnMovement) (CallFunction|MovementMath) false))
    (:then_1
      ;[1 1 1] Animation and Trail Visuals
      (CallFunction|RotateSpaceShipwhenStrafe)
      (Rendering|SetVisibility (Variables|Default|GetNS_Trail_Left) (not (Utilities|Operators|EqualEqual :A (Transformation|GetVelocity))) false))
    (:then_2
      ;[1 1 1] Targeting System
      (CallFunction|TargetingSystem))))

(event Input|MouseEvents|MouseX
  (params (AxisValue :type Float%20%28single-precision%29))
  ;[1 1 1] Setting Inputs Status
  (Pawn|Input|AddControllerYawInput (* AxisValue 0.5)))

(event Input|MouseEvents|MouseY
  (params (AxisValue :type Float%20%28single-precision%29))
  ;[1 1 1] Setting Inputs Status
  (Pawn|Input|AddControllerPitchInput (* (* AxisValue -1.0) 0.5)))

(event Input|KeyboardEvents|A
  (params (Key :type Key%20Structure :default "None"))
  ;[1 1 1] Setting Inputs Status
  (:Pressed
    (Variables|Inputs|SetA_Is_Pressed true))
  (:Released
    (Variables|Inputs|SetA_Is_Pressed false)))

(event Input|KeyboardEvents|D
  (params (Key :type Key%20Structure :default "None"))
  ;[1 1 1] Setting Inputs Status
  (:Pressed
    (Variables|Inputs|SetD_Is_Pressed true))
  (:Released
    (Variables|Inputs|SetD_Is_Pressed false)))

(event Input|KeyboardEvents|W
  (params (Key :type Key%20Structure :default "None"))
  ;[1 1 1] Setting Inputs Status
  (:Pressed
    (Variables|Inputs|SetW_Is_Pressed true))
  (:Released
    (Variables|Inputs|SetW_Is_Pressed false)))

(event Input|KeyboardEvents|S
  (params (Key :type Key%20Structure :default "None"))
  ;[1 1 1] Setting Inputs Status
  (:Pressed
    (Variables|Inputs|SetS_Is_Pressed true))
  (:Released
    (Variables|Inputs|SetS_Is_Pressed false)))

(event Input|KeyboardEvents|LeftCtrl
  (params (Key :type Key%20Structure :default "None"))
  ;[1 1 1] Setting Inputs Status
  (:Pressed
    (Variables|Inputs|SetLeft_Control_Is_Pressed true))
  (:Released
    (Variables|Inputs|SetLeft_Control_Is_Pressed false)))

(event Input|KeyboardEvents|SpaceBar
  (params (Key :type Key%20Structure :default "None"))
  ;[1 1 1] Setting Inputs Status
  (:Pressed
    (Variables|Inputs|SetSpace_Bar_Is_Pressed true))
  (:Released
    (Variables|Inputs|SetSpace_Bar_Is_Pressed false)))

(event Input|KeyboardEvents|LeftShift
  (params (Key :type Key%20Structure :default "None"))
  ;[1 1 1] Setting Inputs Status
  (:Pressed
    (Variables|Movement|SetIs_Sprinting true)
    (Variables|/Script/Engine.FloatingPawnMovement|SetMaxSpeed (Variables|Default|GetFloatingPawnMovement) 2.5e+03)
    (Utilities|Time|UnpauseTimerbyHandle (Variables|Movement|GetStaminaTimerHandle))
    (CallFunction|StartSprintEffect))
  (:Released
    (CallFunction|StopSprinting)))

(event Input|MouseEvents|LeftMouseButton
  (params (Key :type Key%20Structure :default "None"))
  ;[1 1 1] Setting Inputs Status
  (:Pressed
    (Variables|Shooting|SetIsShooting true)
    (CallFunction|LaserShoot))
  (:Released
    (Variables|Shooting|SetIsShooting false)))

(fn ConstructionScript)

(fn MovementMath
  (bind _returnvalue (Transformation|GetActorRightVector))
  (bind _returnvalue_2 (Transformation|GetActorUpVector))
  (bind _returnvalue_3 (Transformation|GetActorForwardVector))
  (Variables|Movement|SetDirection_ForwardBackward (select (or (and (Variables|Inputs|GetW_Is_Pressed) (Variables|Inputs|GetS_Is_Pressed)) (and (not (Variables|Inputs|GetW_Is_Pressed)) (not (Variables|Inputs|GetS_Is_Pressed)))) "0, 0, 0" (Math|Vector|SelectVector (* _returnvalue_3 -1) _returnvalue_3 (Variables|Inputs|GetS_Is_Pressed))))
  (Variables|Movement|SetDirection_LeftRight (select (or (and (Variables|Inputs|GetA_Is_Pressed) (Variables|Inputs|GetD_Is_Pressed)) (and (not (Variables|Inputs|GetA_Is_Pressed)) (not (Variables|Inputs|GetD_Is_Pressed)))) "0, 0, 0" (Math|Vector|SelectVector (* _returnvalue -1) _returnvalue (Variables|Inputs|GetA_Is_Pressed))))
  (Variables|Movement|SetDirection_UpDown (select (or (and (Variables|Inputs|GetLeft_Control_Is_Pressed) (Variables|Inputs|GetSpace_Bar_Is_Pressed)) (and (not (Variables|Inputs|GetLeft_Control_Is_Pressed)) (not (Variables|Inputs|GetSpace_Bar_Is_Pressed)))) "0, 0, 0" (Math|Vector|SelectVector (* _returnvalue_2 -1) _returnvalue_2 (Variables|Inputs|GetLeft_Control_Is_Pressed))))
  (return (+ (Variables|Movement|GetDirection_ForwardBackward) (Variables|Movement|GetDirection_LeftRight) (Variables|Movement|GetDirection_UpDown))))

(fn RotateSpaceShipwhenStrafe
  (bind _body (Variables|Default|GetBody))
  (bind _original_body_relative_rotation (Variables|Movement|GetOriginal%20Body%20Relative%20Rotation))
  (bind _body_2 (Variables|Default|GetBody))
  (if (or (and (Variables|Inputs|GetA_Is_Pressed) (Variables|Inputs|GetD_Is_Pressed)) (and (not (Variables|Inputs|GetA_Is_Pressed)) (not (Variables|Inputs|GetD_Is_Pressed))))
    (Transformation|SetRelativeRotation _body_2 (Math|Interpolation|RInterpTo (Variables|/Script/Engine.SceneComponent|GetRelativeRotation _body_2) (Variables|Movement|GetOriginal%20Body%20Relative%20Rotation) (Utilities|Time|GetWorldDeltaSeconds) 1.0) false false)
    (else
      (Transformation|SetRelativeRotation _body (Math|Interpolation|RInterpTo (Variables|/Script/Engine.SceneComponent|GetRelativeRotation _body) (Math|Rotator|CombineRotators (Variables|Movement|GetOriginal%20Body%20Relative%20Rotation) (Math|Rotator|SelectRotator (Math|Rotator|CombineRotators _original_body_relative_rotation "0.000000,0.000000,-15.000000") (Math|Rotator|CombineRotators _original_body_relative_rotation "0.000000,0.000000,15.000000") (Variables|Inputs|GetA_Is_Pressed))) (Utilities|Time|GetWorldDeltaSeconds) 1.0) false false))))

(fn SetDefaults
  (Variables|Movement|SetOriginal%20Body%20Relative%20Rotation (Variables|/Script/Engine.SceneComponent|GetRelativeRotation (Variables|Default|GetBody)))
  (Variables|Movement|SetCurrentStamina (Variables|Movement|GetMaxStamina)))

(fn StopSprinting
  (Variables|Movement|SetIs_Sprinting false)
  (Variables|/Script/Engine.FloatingPawnMovement|SetMaxSpeed (Variables|Default|GetFloatingPawnMovement) 1.2e+03)
  (CallFunction|StopSprintEffect))

(fn TargetingSystem
  (bind _camera (Variables|Default|GetCamera))
  (bind _output_get (Variables|Shooting|SetTarget (+ (Transformation|GetWorldLocation _camera) (* (Math|Vector|GetForwardVector _camera) (Variables|Shooting|GetRange_of_Primary_Fire)))))
  (bind (_outhit _returnvalue) (Collision|SphereTraceForObjects (Transformation|GetWorldLocation (Variables|Default|GetCamera)) _output_get 2e+01 (Variables|Shooting|GetObject%20Types) false 0 "None"))
  (if _returnvalue
    (Variables|Shooting|SetTarget (.Location (Collision|BreakHitResult _outhit)))
    (Variables|Shooting|SetTarget%20Actor (.HitActor (Collision|BreakHitResult _outhit)))
    (Default|HasTarget (Variables|Default|GetWG_Gameplay_Ref))
    (else
      (Variables|Shooting|SetTarget%20Actor 0)
      (Default|HasNoTarget (Variables|Default|GetWG_Gameplay_Ref)))))

(fn DirectionCalculation
  (params (Target :type Scene%20Component%20Object%20Reference))
  (bind _returnvalue (Transformation|GetWorldLocation Target))
  (return (Math|Vector|Normalize (- (+ _returnvalue (- (Variables|Shooting|GetTarget) _returnvalue)) (Transformation|GetWorldLocation Target)))))

(fn SpawnLaser
  (params (MuzzlePoint :type Scene%20Component%20Object%20Reference))
  (bind _returnvalue (Game|SpawnActorfromClass "/Game/Blueprints/BP_PlayerBullet.BP_PlayerBullet_C" (Transformation|GetWorldTransform MuzzlePoint) "Undefined" "MultiplyWithRoot" 0 0))
  (Default|BulletonSpawn _returnvalue (CallFunction|DirectionCalculation MuzzlePoint)))