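; Base enemy actor that damages what it collides with and explodes when it dies.
; An overlap between EnemyBody and a component tagged "Body" applies CollisionDamage to the other actor, then kills the enemy.
; An UpdateOwner event with a Dead flag also triggers death.
; Both paths share a Death function that spawns a scaled-up explosion emitter at the actor's location and destroys it.
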(event OnComponentBeginOverlap(EnemyBody)
  (params (OverlappedComponent :type Primitive%20Component%20Object%20Reference) (OtherActor :type Actor%20Object%20Reference) (OtherComp :type Primitive%20Component%20Object%20Reference) (OtherBodyIndex :type Integer) (bFromSweep :type Boolean) (SweepResult :type Hit%20Result%20Structure%20%28by%20ref%29))
  (Utilities|IsValid OtherActor
    (:Is%20Valid
      (if (Components|ComponentHasTag OtherComp "Body")
        (Game|Damage|ApplyDamage OtherActor (Variables|Default|GetCollisionDamage) 0 0)
        (CallFunction|Death)))))

(event EventUpdateOwner
  (params (Health :type Float%20%28double-precision%29) (Dead :type Boolean))
  (if Dead
    (CallFunction|Death)))

(fn ConstructionScript)

(fn Death
  (Effects|SpawnEmitteratLocation "/Game/Particles/P_Explosion.P_Explosion" (Transformation|GetActorLocation) "0, 0, 0" "5.000000,5.000000,5.000000")
  (Actor|DestroyActor))