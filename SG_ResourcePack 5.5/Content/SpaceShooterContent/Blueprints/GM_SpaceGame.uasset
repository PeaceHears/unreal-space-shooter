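; GM_SpaceGame is the space shooter's game mode, handling the main menu and player ship spawning.
; On BeginPlay it creates the WG_MainMenu widget, stores a reference and shows it with the cursor visible and UI-only input.
; HideMainMenu reverses this to game-only input, and SpawnPlayer spawns BP_PlayerSpaceShip.
; Neither of those two events is called within this Blueprint.
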(event Custom|Show%20Main%20Menu
  (bind _returnvalue (Game|GetPlayerController 0))
  (bind _wg_mainmenu_ref (Variables|Default|GetWG%20MainMenu%20Ref))
  (Variables|/Script/Engine.PlayerController|SetbShowMouseCursor _returnvalue true)
  (Input|SetInputModeUIOnly _returnvalue _wg_mainmenu_ref "DoNotLock" false)
  (UserInterface|Viewport|AddtoViewport _wg_mainmenu_ref 0))

(event Custom|Hide%20Main%20Menu
  (bind _returnvalue (Game|GetPlayerController 0))
  (Variables|/Script/Engine.PlayerController|SetbShowMouseCursor _returnvalue false)
  (Input|SetInputModeGameOnly _returnvalue false)
  (Widget|RemovefromParent (Variables|Default|GetWG%20MainMenu%20Ref)))

(event Custom|Spawn%20Player
  (Game|SpawnActorfromClass "/Game/SpaceShooterContent/Blueprints/BP_PlayerSpaceShip.BP_PlayerSpaceShip_C" (Math|Transform|MakeTransform "0, 0, 0" "0, 0, 0" "1.000000,1.000000,1.000000") "Undefined" "MultiplyWithRoot" 0 0))

(event EventBeginPlay
  (bind _returnvalue (UserInterface|CreateWidget "/Game/SpaceShooterContent/UI/WG_MainMenu.WG_MainMenu_C" (Game|GetPlayerController 0)))
  (Variables|Default|SetWG%20MainMenu%20Ref _returnvalue)
  (CallFunction|ShowMainMenu))

(fn ConstructionScript)