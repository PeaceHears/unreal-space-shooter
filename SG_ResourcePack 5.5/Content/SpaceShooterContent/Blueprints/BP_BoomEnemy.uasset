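; BP_BoomEnemy is a space shooter enemy that homes in on the player.
; Every tick it turns toward the player through RotateTowardsPlayer and moves at constant Speed toward the player pawn using VInterpToConstant, without sweep.
; On BeginPlay it binds RotatingMovement to EnemyBody, so that component spins separately from the actor's facing.
; The construction script only calls the parent, and no explosion logic appears in these graphs.
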(event EventBeginPlay
  (Components|Movement|SetUpdatedComponent (Variables|Default|GetRotatingMovement) (Variables|Default|GetEnemyBody)))

(event EventTick
  (params (DeltaSeconds :type Float%20%28single-precision%29))
  (CallFunction|RotateTowardsPlayer (Game|GetPlayerController 0) self DeltaSeconds 1e+01)
  (Transformation|SetActorLocation (Math|Interpolation|VInterptoConstant (Transformation|GetActorLocation) (Transformation|GetActorLocation (Game|Player|GetPlayerPawn 0)) DeltaSeconds (Math|Conversions|ToFloat(Integer) (Variables|Default|GetSpeed))) false false))

(fn ConstructionScript
  (|CallParentFunction))