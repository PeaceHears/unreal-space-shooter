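; BPC_Damageable is an actor component that gives its owner health in the space shooter.
; On BeginPlay it binds to the owner's OnTakeAnyDamage event and subtracts incoming damage from CurrentHealth.
; IncreaseHealth and DecreaseHealth clamp health between zero and MaxHealth, then send the new value and a dead flag to the owner through UpdateOwnerMessage, leaving the reaction to the owner.
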(event Custom|BindOnTakeAnyDamage
  (params (DamagedActor :type Actor%20Object%20Reference) (Damage :type Float%20%28single-precision%29) (DamageType :type Damage%20Type%20Object%20Reference) (InstigatedBy :type Controller%20Object%20Reference) (DamageCauser :type Actor%20Object%20Reference))
  (CallFunction|DecreaseHealth Damage))

(event EventBeginPlay
  (EventDispatchers|BindEventtoOnTakeAnyDamage (Components|GetOwner) (delegate Custom|BindOnTakeAnyDamage)))

(event EventTick
  (params (DeltaSeconds :type Float%20%28single-precision%29)))

(fn IncreaseHealth
  (params (HealAmount :type Float%20%28double-precision%29))
  (Variables|Default|SetCurrentHealth (Math|Float|Clamp(Float) (+ HealAmount (Variables|Default|GetCurrentHealth)) 0.0 (Variables|Default|GetMaxHealth)))
  (Class|BICommunications|UpdateOwner(Message) (Components|GetOwner) (Variables|Default|GetCurrentHealth) (== (Variables|Default|GetCurrentHealth) 0.0)))

(fn DecreaseHealth
  (params (Damage :type Float%20%28double-precision%29))
  (Variables|Default|SetCurrentHealth (Math|Float|Clamp(Float) (- (Variables|Default|GetCurrentHealth) Damage) 0.0 (Variables|Default|GetMaxHealth)))
  (Class|BICommunications|UpdateOwner(Message) (Components|GetOwner) (Variables|Default|GetCurrentHealth) (== (Variables|Default|GetCurrentHealth) 0.0)))