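; Homing missile projectile that explodes on touching an Enemy-tagged actor, damaging all enemies in its damage area.
; LaunchMissile either chases a given enemy target by interpolating location on Tick, or fires straight with a detector collision enabled.
; The detector hands the first enemy found to ProjectileMovement homing; losing a Tick-chased target re-enables detection, with resettable DoOnce gates limiting retargeting.
; Death spawns an explosion emitter and destroys the missile.
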(event OnComponentBeginOverlap(HomingDetectorCollision)
  (params (OverlappedComponent :type Primitive%20Component%20Object%20Reference) (OtherActor :type Actor%20Object%20Reference) (OtherComp :type Primitive%20Component%20Object%20Reference) (OtherBodyIndex :type Integer) (bFromSweep :type Boolean) (SweepResult :type Hit%20Result%20Structure%20%28by%20ref%29))
  (if (Actor|ActorHasTag OtherActor "Enemy")
    (Utilities|FlowControl|DoOnce (Variables|Default|GetCustomHoming)
      (:Completed
        (CallFunction|ResetSearchforTarget)
        (Variables|Default|SetTarget OtherActor)
        (CallFunction|SetHoming)))))

(event OnComponentBeginOverlap(ExplodeDetection)
  (params (OverlappedComponent :type Primitive%20Component%20Object%20Reference) (OtherActor :type Actor%20Object%20Reference) (OtherComp :type Primitive%20Component%20Object%20Reference) (OtherBodyIndex :type Integer) (bFromSweep :type Boolean) (SweepResult :type Hit%20Result%20Structure%20%28by%20ref%29))
  (if (Actor|ActorHasTag OtherActor "Enemy")
    (Utilities|FlowControl|DoOnce false
      (:Completed
        (CallFunction|ApplyAOEDamage)))))

(event Custom|ResetCollision
  (Utilities|FlowControl|DoOnce (Variables|Default|GetCustomHoming)) ; enters at Reset
)

(event Custom|ResetSearchForTarget
  (Utilities|FlowControl|DoOnce false) ; enters at Reset
)

(event Custom|LaunchMissile
  (params (Velocity :type Vector) (TargetActor :type Actor%20Object%20Reference))
  (Variables|Default|SetTargetVelocity Velocity)
  (bind _output_get (Variables|Default|SetTarget TargetActor))
  (Utilities|IsValid _output_get
    (:Is%20Valid
      (if (Actor|ActorHasTag (Variables|Default|GetTarget) "Enemy")
        (Variables|Default|SetCustomHoming true)
        (else
          (Variables|/Script/Engine.MovementComponent|SetVelocity (Variables|Default|GetProjectileMovement) (* (Variables|Default|GetTargetVelocity) 20000) :!label _label)
          (Variables|/Script/Engine.PrimitiveComponent|SetbGenerateOverlapEvents (Variables|Default|GetHomingDetectorCollision) true))))
    (:Is%20Not%20Valid
      (goto _label))))

(event EventBeginPlay)

(event Collision|EventActorBeginOverlap
  (params (OtherActor :type Actor%20Object%20Reference)))

(event EventTick
  (params (DeltaSeconds :type Float%20%28single-precision%29))
  (if (Variables|Default|GetCustomHoming)
    (Utilities|IsValid (Variables|Default|GetTarget)
      (:Is%20Valid
        (Transformation|SetActorLocation (Math|Interpolation|VInterptoConstant (Transformation|GetActorLocation) (Transformation|GetActorLocation (Variables|Default|GetTarget)) DeltaSeconds 5e+04) false false))
      (:Is%20Not%20Valid
        (Utilities|FlowControl|DoOnce false
          (:Completed
            (Variables|Default|SetCustomHoming false)
            (Variables|/Script/Engine.PrimitiveComponent|SetbGenerateOverlapEvents (Variables|Default|GetHomingDetectorCollision) true)
            (CallFunction|ResetCollision)))))))

(fn ConstructionScript)

(fn ApplyAOEDamage
  (for _array_element (Collision|GetOverlappingActors (Variables|Default|GetDamageArea) 0 :!class /Script/Engine.PrimitiveComponent)
    (if (Actor|ActorHasTag _array_element "Enemy")
      (Game|Damage|ApplyDamage _array_element 5.0 0 0)))
  (CallFunction|Death))

(fn SetHoming
  (bind _projectilemovement (Variables|Default|GetProjectileMovement))
  (Variables|/Script/Engine.MovementComponent|SetVelocity _projectilemovement "0, 0, 0")
  (Variables|/Script/Engine.ProjectileMovementComponent|SetbIsHomingProjectile _projectilemovement true)
  (Variables|/Script/Engine.ProjectileMovementComponent|SetHomingTargetComponent _projectilemovement (Actor|GetComponentbyClass (Variables|Default|GetTarget) "/Script/Engine.SceneComponent")))

(fn Death
  (Effects|SpawnEmitteratLocation "/Game/StarterContent/Particles/P_Explosion.P_Explosion" (Transformation|GetActorLocation) "0, 0, 0" "20.000000,20.000000,20.000000")
  (Actor|DestroyActor))