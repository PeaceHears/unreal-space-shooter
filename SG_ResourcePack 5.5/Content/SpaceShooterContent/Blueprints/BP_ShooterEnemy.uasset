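; BP_ShooterEnemy is a space shooter enemy that repositions around the player and fires bursts of BP_EnemyBullet while turning to face them.
; After a short startup delay, it picks a random point in a distance band around the player and glides there at constant speed with sweep.
; On arrival, a DoOnce starts a recursive, delayed Shoot loop firing three muzzles, one aimed and two scattered.
; When the burst ends, it picks a new location, which re-arms the DoOnce.
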(event Custom|Shoot
  (bind _returnvalue (Game|Player|GetPlayerPawn 0))
  (bind _returnvalue_2 (Transformation|GetActorLocation _returnvalue))
  (bind _returnvalue_3 (Math|Random|RandomPointinBoundingBox _returnvalue_2 "500.000000,500.000000,500.000000"))
  (if (== (Variables|Default|GetCurrentShot) (Variables|Default|GetMaxShots))
    (Variables|Default|SetCurrentShot 0)
    (CallFunction|SelectMoveLocation)
    (else
      (Variables|Default|SetCurrentShot (+ (Variables|Default|GetCurrentShot) 1))
      (Utilities|IsValid (Game|Player|GetPlayerPawn 0)
        (:Is%20Valid
          (Utilities|FlowControl|Sequence
            (:then_0
              (CallFunction|ShootBullet (Variables|Default|GetMuzzle1) (Transformation|GetActorLocation (Game|Player|GetPlayerPawn 0))))
            (:then_1
              (CallFunction|ShootBullet (Variables|Default|GetMuzzle2) _returnvalue_3))
            (:then_2
              (CallFunction|ShootBullet (Variables|Default|GetMuzzle3) _returnvalue_3))
            (:then_3
              (Utilities|FlowControl|Delay 0.2)
              (CallFunction|Shoot))))))))

(event Custom|ResetShoot
  (Utilities|FlowControl|DoOnce false) ; enters at Reset
)

(event EventBeginPlay
  (Utilities|FlowControl|Delay 3.0)
  (CallFunction|SelectMoveLocation))

(event EventTick
  (params (DeltaSeconds :type Float%20%28single-precision%29))
  (CallFunction|RotateTowardsPlayer (Game|GetPlayerController 0) self DeltaSeconds 5.0)
  (if (Variables|Default|GetIsMoving)
    (Transformation|SetActorLocation (Math|Interpolation|VInterptoConstant (Transformation|GetActorLocation) (Variables|Default|GetTargetLocation) DeltaSeconds (Math|Conversions|ToFloat(Integer) (Variables|Default|GetSpeed))) true false)
    (if (Utilities|Operators|EqualEqual (Transformation|GetActorLocation) (Variables|Default|GetTargetLocation) 1.0)
      (Variables|Default|SetIsMoving false)
      (Utilities|FlowControl|DoOnce false
        (:Completed
          (CallFunction|Shoot))))))

(fn ConstructionScript
  (|CallParentFunction))

(fn SelectMoveLocation
  (bind _returnvalue (Game|Player|GetPlayerPawn 0))
  (CallFunction|ResetShoot)
  (Utilities|IsValid _returnvalue
    (:Is%20Valid
      (Variables|Default|SetTargetLocation (+ (Transformation|GetActorLocation _returnvalue) (* (Math|Random|RandomUnitVector) (Math|Random|RandomIntegerinRange 2000 3500))))
      (Variables|Default|SetIsMoving true))))

(fn ShootBullet
  (params (From :type Scene%20Component%20Object%20Reference) (Target :type Vector%20%28by%20ref%29))
  (bind _returnvalue (Transformation|GetWorldLocation From))
  (bind _returnvalue_2 (Game|SpawnActorfromClass "/Game/SpaceShooterContent/Blueprints/BP_EnemyBullet.BP_EnemyBullet_C" (Math|Transform|MakeTransform _returnvalue "0, 0, 0" "1.000000,1.000000,1.000000") "Undefined" "MultiplyWithRoot" 0 0))
  (Default|BulletonSpawn _returnvalue_2 (Math|Vector|GetForwardVector (Math|Rotator|FindLookatRotation _returnvalue Target))))