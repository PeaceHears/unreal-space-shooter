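; BP_PlayerBullet is the player's laser projectile in the space shooter, damaging enemies it touches.
; A BulletOnSpawn event sets the ProjectileMovement velocity from a passed-in direction and the bullet speed.
; When the LaserBullet component begins overlapping an actor tagged Enemy, it applies fixed damage, spawns an explosion emitter at the bullet's location and destroys itself.
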(event OnComponentBeginOverlap(LaserBullet)
  (params (OverlappedComponent :type Primitive%20Component%20Object%20Reference) (OtherActor :type Actor%20Object%20Reference) (OtherComp :type Primitive%20Component%20Object%20Reference) (OtherBodyIndex :type Integer) (bFromSweep :type Boolean) (SweepResult :type Hit%20Result%20Structure%20%28by%20ref%29))
  (if (Actor|ActorHasTag OtherActor "Enemy")
    (Game|Damage|ApplyDamage OtherActor 2.0 0 0)
    (Effects|SpawnEmitteratLocation "/Game/SpaceShooterContent/Particles/P_Explosion.P_Explosion" (Transformation|GetActorLocation))
    (Actor|DestroyActor)))

(event Custom|BulletOnSpawn
  (params (Direction :type Vector))
  (Variables|/Script/Engine.MovementComponent|SetVelocity (Variables|Default|GetProjectileMovement) (* Direction (Variables|Default|GetBulletSpeed))))

(fn ConstructionScript)